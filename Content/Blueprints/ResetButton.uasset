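; ResetButton is a Blueprint that returns ImpulseCube actors to their start positions.
; It caches all ImpulseCube actors on BeginPlay.
; Its ResetPosition event loops through them, disabling physics on each body and moving it to that cube's StartPosition.
; A short Delay inside the loop precedes re-enabling physics; since the loop does not wait for it, only the last cube regains simulation.
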(event `self.ReceiveBeginPlay`
  (bind _outactors (`GameplayStatics.GetAllActorsOfClass` "/Game/StarterContent/Blueprints/Assets/ImpulseCube.ImpulseCube_C"))
  (set `self.ResetObjects` _outactors))

(event `ResetPosition`
  (for _array_element (`self.ResetObjects`)
    (bind _asimpulse_cube (cast `/Game/StarterContent/Blueprints/Assets/ImpulseCube` _array_element))
    (bind _physicsbody (`/Game/StarterContent/Blueprints/Assets/ImpulseCube.PhysicsBody` _asimpulse_cube))
    (`PrimitiveComponent.SetSimulatePhysics` _physicsbody false)
    (`SceneComponent.K2_SetWorldLocation` _physicsbody (`/Game/StarterContent/Blueprints/Assets/ImpulseCube.StartPosition` _asimpulse_cube) false false)
    (`KismetSystemLibrary.Delay` 0.2)
    (`PrimitiveComponent.SetSimulatePhysics` _physicsbody true)))

(fn `UserConstructionScript`)